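; BP_MenuControl is a control menu Blueprint that toggles the visibility of every BP_Horn in the level.
; On BeginPlay it creates a W_MenuControl widget, assigns it to its Widget component and binds to the CheckBox1 state change.
; Each change finds all BP_Horn actors, then shows or hides their Widget and Plane components and switches their collision between QueryAndPhysics and NoCollision to match.
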(event Custom|SetVisible
  (params (bIsChecked :type Boolean))
  (bind _returnvalue (not bIsChecked))
  (bind _outactors (Actor|GetAllActorsOfClass "/Game/MyStuff/Drawable/BP_Horn.BP_Horn_C"))
  (for _array_element _outactors
    (bind _asbp_horn (Utilities|Casting|CastToBP_Horn _array_element))
    (Development|SetHiddeninGame (Variables|/Game/MyStuff/Drawable/BP_Horn.BP_Horn_C|GetWidget _asbp_horn) _returnvalue false)
    (if _returnvalue
      (Collision|SetCollisionEnabled (Variables|/Game/MyStuff/Drawable/BP_Horn.BP_Horn_C|GetPlane _asbp_horn) "NoCollision")
      (else
        (Collision|SetCollisionEnabled (Variables|/Game/MyStuff/Drawable/BP_Horn.BP_Horn_C|GetWidget _asbp_horn) "QueryAndPhysics")))))

(event EventBeginPlay
  (bind _returnvalue (UserInterface|CreateWidget "/Game/MyStuff/Widgets/W_MenuControl.W_MenuControl_C"))
  (bind _output_get (Variables|Default|SetWidgetRef _returnvalue))
  (UserInterface|SetWidget (Variables|Default|GetWidget) _output_get)
  (EventDispatchers|BindEventtoOnCheckStateChanged (Variables|/Game/MyStuff/Widgets/W_MenuControl.W_MenuControl_C|GetCheckBox_1 (Variables|Default|GetWidgetRef)) (delegate Custom|SetVisible)))

(fn ConstructionScript)