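; BP_Horn is a placeable drawable image actor, shown on a Cube mesh, with controls to resize, rotate or delete it.
; BeginPlay creates a W_AdjustImage widget, assigns it to the Widget component and binds its two value controls and button.
; The values scale the cube in X and Z with zero Y thickness and set its world pitch, while the button destroys the actor.
; The construction script stores a dynamic material instance of the cube.
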(event Custom|SetSize
  (params (Value :type Float%20%28single-precision%29))
  (bind _returnvalue (* Value 2.0))
  (Transformation|SetRelativeScale3D (Variables|Default|GetCube) (Math|Vector|MakeVector _returnvalue 0.0 _returnvalue)))

(event Custom|SetRotation
  (params (Value :type Float%20%28single-precision%29))
  (Transformation|SetWorldRotation (Variables|Default|GetCube) (Math|Rotator|MakeRotator 0.0 (* Value 3.6e+02) 0.0) false false))

(event Custom|DestroyImage
  (Actor|DestroyActor))

(event EventBeginPlay
  (bind _returnvalue (UserInterface|CreateWidget "/Game/MyStuff/Widgets/W_AdjustImage.W_AdjustImage_C"))
  (bind _output_get (Variables|Default|SetWidgetRef _returnvalue))
  (UserInterface|SetWidget (Variables|Default|GetWidget) _output_get)
  (EventDispatchers|BindEventtoOnValueChanged (Variables|/Game/MyStuff/Widgets/W_AdjustImage.W_AdjustImage_C|GetSize (Variables|Default|GetWidgetRef)) (delegate Custom|SetSize))
  (EventDispatchers|BindEventtoOnValueChanged (Variables|/Game/MyStuff/Widgets/W_AdjustImage.W_AdjustImage_C|GetRotate (Variables|Default|GetWidgetRef)) (delegate Custom|SetRotation))
  (EventDispatchers|BindEventtoOnClicked (Variables|/Game/MyStuff/Widgets/W_AdjustImage.W_AdjustImage_C|GetButton_16 (Variables|Default|GetWidgetRef)) (delegate Custom|DestroyImage)))

(fn ConstructionScript
  (bind _returnvalue (Rendering|Material|CreateDynamicMaterialInstance (Variables|Default|GetCube) 0 (Variables|Default|GetSourceMaterial) "None" :!class /Script/Engine.PrimitiveComponent))
  (Variables|Default|SetMatRef _returnvalue))