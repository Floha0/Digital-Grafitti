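; BP_DrawableSetting is an actor that hosts a W_Drawables widget for picking a drawable image and spawning it into the level.
; Left and right buttons cycle a wrapping index between DevilHorns and Wolf textures, updating the preview and the current texture.
; The Spawn button creates a BP_Horn at a hard-coded location and passes that texture to its material's DrawableImg parameter.
; Disconnected material-swap and brush-preview nodes remain unused.
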(event Custom|Spawn
  (bind _returnvalue (Game|SpawnActorfromClass "/Game/MyStuff/Drawable/BP_Horn.BP_Horn_C" (Math|Transform|MakeTransform "-1235.000000,95.000000,257.000000" "0, 0, 0" "1.000000,1.000000,1.000000") "Undefined" 0 0))
  (Rendering|Material|SetTextureParameterValue (Variables|/Game/MyStuff/Drawable/BP_Horn.BP_Horn_C|GetMatRef _returnvalue) "DrawableImg" (Variables|Default|GetCurrentTex)))

(event Custom|BrushTip_Right
  (bind _wbp_brushsetting (Variables|Default|GetWBP_BrushSetting))
  (bind _brushpreview (Variables|/Game/MyStuff/Widgets/W_Drawables.W_Drawables_C|GetBrushPreview _wbp_brushsetting))
  (bind _result (Math|Integer|IncrementInt (Variables|Default|GetBrushTipShapeIndex))
    (:%20%20
      (if (> _result 1)
        (Variables|Default|SetBrushTipShapeIndex 0))
      (switch int (Variables|Default|GetBrushTipShapeIndex)
        (:0
          (Appearance|SetBrushfromTexture _brushpreview "/Game/MyStuff/Drawable/DevilHorns.DevilHorns" false)
          (Variables|Default|SetCurrentTex "/Game/MyStuff/Drawable/DevilHorns.DevilHorns"))
        (:1
          (Appearance|SetBrushfromTexture _brushpreview "/Game/MyStuff/Drawable/Wolf.Wolf" false)
          (Variables|Default|SetCurrentTex "/Game/MyStuff/Drawable/Wolf.Wolf"))))))

(event Custom|BrushTip_Left
  (bind _wbp_brushsetting (Variables|Default|GetWBP_BrushSetting))
  (bind _brushpreview (Variables|/Game/MyStuff/Widgets/W_Drawables.W_Drawables_C|GetBrushPreview _wbp_brushsetting))
  (bind _result (Math|Integer|DecrementInt (Variables|Default|GetBrushTipShapeIndex))
    (:%20%20
      (if (< _result 0)
        (Variables|Default|SetBrushTipShapeIndex 1))
      (switch int (Variables|Default|GetBrushTipShapeIndex)
        (:0
          (Appearance|SetBrushfromTexture _brushpreview "/Game/MyStuff/Drawable/DevilHorns.DevilHorns" false)
          (Variables|Default|SetCurrentTex "/Game/MyStuff/Drawable/DevilHorns.DevilHorns"))
        (:1
          (Appearance|SetBrushfromTexture _brushpreview "/Game/MyStuff/Drawable/Wolf.Wolf" false)
          (Variables|Default|SetCurrentTex "/Game/MyStuff/Drawable/Wolf.Wolf"))))))

(event EventBeginPlay
  (bind _returnvalue (UserInterface|CreateWidget "/Game/MyStuff/Widgets/W_Drawables.W_Drawables_C"))
  (bind _output_get (Variables|Default|SetWBP_BrushSetting _returnvalue))
  (UserInterface|SetWidget (Variables|Default|GetWidget) _output_get)
  (EventDispatchers|BindEventtoOnClicked (Variables|/Game/MyStuff/Widgets/W_Drawables.W_Drawables_C|GetBrushTip_RightButton (Variables|Default|GetWBP_BrushSetting)) (delegate Custom|BrushTip_Right))
  (EventDispatchers|BindEventtoOnClicked (Variables|/Game/MyStuff/Widgets/W_Drawables.W_Drawables_C|GetBrushTip_LeftButton (Variables|Default|GetWBP_BrushSetting)) (delegate Custom|BrushTip_Left))
  (EventDispatchers|BindEventtoOnClicked (Variables|/Game/MyStuff/Widgets/W_Drawables.W_Drawables_C|GetSpawn_Button (Variables|Default|GetWBP_BrushSetting)) (delegate Custom|Spawn)))

(fn ConstructionScript)