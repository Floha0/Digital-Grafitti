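; Brush settings panel actor for a VR drawing toolkit, hosting WBP_BrushSetting in a widget component to control the first BP_Pen found.
; Slider and button events set the pen's size, rotation, opacity and five cycling tip textures, mirroring each on the widget preview.
; Picker X/Y inputs become hue (angle) and saturation (radius), combined with the value slider for brush color.
; Tick moves DotPoint to the pen's picked color position.
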(event Custom|Picker%20Color%20Y
  (params (Y :type Float%20%28double-precision%29))
  ;[1 1 1] Binding Brush Setting Widget Events and Adujusting Values of them
  ;;[1 1 1] Color Picker Event
  (bind _output_get (Variables|Default|SetY%20Aixs (* Y -1.0)))
  (bind _output_get_2 (Variables|Default|SetClamp%20Y (Math|Float|MapRangeClamped _output_get 0.0 -1.0 -1.0 1.0))))

(event Custom|Picker%20Color%20X
  (params (X :type Float%20%28double-precision%29))
  ;[1 1 1] Binding Brush Setting Widget Events and Adujusting Values of them
  ;;[1 1 1] Color Picker Event
  (bind _output_get (Variables|Default|SetX%20Aixs X))
  (bind _output_get_2 (Variables|Default|SetClamp%20X (Math|Float|MapRangeClamped _output_get 0.0 1.0 -1.0 1.0)))
  (Variables|Default|SetDegree (Class|KismetMathLibrary|DegAtan2 (stale Custom|Picker%20Color%20Y _output_get_2) _output_get_2))
  (bind _output_get_3 (Variables|Default|SetCurrent%20Vector (Math|Vector2D|MakeVector2D (Variables|Default|GetClamp%20X) (Variables|Default|GetClamp%20Y))))
  (Variables|Default|SetVector%20Size (Math|Vector2D|Vector2DLength _output_get_3))
  (if (< (Variables|Default|GetDegree) 0.0)
    (bind _output_get_4 (Variables|Default|SetPicked%20Color (Class|KismetMathLibrary|HSVtoRGB (Math|Float|MapRangeClamped (Variables|Default|GetDegree) -1.8e+02 0.0 1.8e+02 3.6e+02) (Variables|Default|GetVector%20Size) (Variables|Default|GetColorValue) 1.0)))
    (Rendering|Material|SetVectorParameterValue (Variables|/Game/DrawingToolkit/Blueprint/BP_Pen.BP_Pen_C|GetBrushMaterial (Variables|Default|GetBP%20Pen)) "Brush Color" _output_get_4 :!class /Script/Engine.MaterialInstanceDynamic)
    (Class|Image|SetBrushTintColor (Variables|/Game/DrawingToolkit/Blueprint/WidgetBP/WBP_BrushSetting.WBP_BrushSetting_C|GetBrushPreview (Variables|Default|GetWBP_BrushSetting)) (Utilities|Struct|MakeSlateColor (Class|KismetMathLibrary|HSVtoRGB (Math|Float|MapRangeClamped (Variables|Default|GetDegree) -1.8e+02 0.0 1.8e+02 3.6e+02) (Variables|Default|GetVector%20Size) (Variables|Default|GetColorValue) 1.0) "UseColor_Specified"))
    (Class|Image|SetBrushTintColor (Variables|/Game/DrawingToolkit/Blueprint/WidgetBP/WBP_BrushSetting.WBP_BrushSetting_C|GetColorValueBack (Variables|Default|GetWBP_BrushSetting)) (Utilities|Struct|MakeSlateColor (Class|KismetMathLibrary|HSVtoRGB (Math|Float|MapRangeClamped (Variables|Default|GetDegree) -1.8e+02 0.0 1.8e+02 3.6e+02) (Variables|Default|GetVector%20Size) 1.0 1.0) "UseColor_Specified"))
    (else
      (bind _output_get_5 (Variables|Default|SetPicked%20Color (Class|KismetMathLibrary|HSVtoRGB (Variables|Default|GetDegree) (Variables|Default|GetVector%20Size) (Variables|Default|GetColorValue) 1.0)))
      (Rendering|Material|SetVectorParameterValue (Variables|/Game/DrawingToolkit/Blueprint/BP_Pen.BP_Pen_C|GetBrushMaterial (Variables|Default|GetBP%20Pen)) "Brush Color" _output_get_5 :!class /Script/Engine.MaterialInstanceDynamic)
      (Class|Image|SetBrushTintColor (Variables|/Game/DrawingToolkit/Blueprint/WidgetBP/WBP_BrushSetting.WBP_BrushSetting_C|GetBrushPreview (Variables|Default|GetWBP_BrushSetting)) (Utilities|Struct|MakeSlateColor (Class|KismetMathLibrary|HSVtoRGB (Variables|Default|GetDegree) (Variables|Default|GetVector%20Size) (Variables|Default|GetColorValue) 1.0) "UseColor_Specified"))
      (Class|Image|SetBrushTintColor (Variables|/Game/DrawingToolkit/Blueprint/WidgetBP/WBP_BrushSetting.WBP_BrushSetting_C|GetColorValueBack (Variables|Default|GetWBP_BrushSetting)) (Utilities|Struct|MakeSlateColor (Class|KismetMathLibrary|HSVtoRGB (Variables|Default|GetDegree) (Variables|Default|GetVector%20Size) 1.0 1.0) "UseColor_Specified")))))

(event Custom|BrushSize
  (params (Value :type Float%20%28single-precision%29))
  (bind _returnvalue (Math|Float|MapRangeClamped Value 0.0 1.0 15.0 256.0))
  ;[1 1 1] Binding Brush Setting Widget Events and Adujusting Values of them
  (Variables|/Game/DrawingToolkit/Blueprint/BP_Pen.BP_Pen_C|SetBrushSize (Variables|Default|GetBP%20Pen) (Math|Float|MapRangeClamped Value 0.0 1.0 0.02 0.6))
  (Class|Image|SetDesiredSizeOverride (Variables|/Game/DrawingToolkit/Blueprint/WidgetBP/WBP_BrushSetting.WBP_BrushSetting_C|GetBrushPreview (Variables|Default|GetWBP_BrushSetting)) (Math|Vector2D|MakeVector2D _returnvalue _returnvalue)))

(event Custom|BrushOpacity
  (params (Value :type Float%20%28single-precision%29))
  (bind _returnvalue (Math|Float|MapRangeClamped Value 0.0 1.0 0.01 1.0))
  ;[1 1 1] Binding Brush Setting Widget Events and Adujusting Values of them
  (Rendering|Material|SetScalarParameterValue (Variables|/Game/DrawingToolkit/Blueprint/BP_Pen.BP_Pen_C|GetBrushMaterial (Variables|Default|GetBP%20Pen)) "Opacity" _returnvalue :!class /Script/Engine.MaterialInstanceDynamic)
  (Class|Image|SetOpacity (Variables|/Game/DrawingToolkit/Blueprint/WidgetBP/WBP_BrushSetting.WBP_BrushSetting_C|GetBrushPreview (Variables|Default|GetWBP_BrushSetting)) _returnvalue))

(event Custom|BrushTip_Right
  (bind _wbp_brushsetting (Variables|Default|GetWBP_BrushSetting))
  (bind _bp_pen (Variables|Default|GetBP%20Pen))
  (bind _brushname (Variables|/Game/DrawingToolkit/Blueprint/WidgetBP/WBP_BrushSetting.WBP_BrushSetting_C|GetBrushName _wbp_brushsetting))
  (bind _brushmaterial (Variables|/Game/DrawingToolkit/Blueprint/BP_Pen.BP_Pen_C|GetBrushMaterial _bp_pen))
  (bind _brushpreview (Variables|/Game/DrawingToolkit/Blueprint/WidgetBP/WBP_BrushSetting.WBP_BrushSetting_C|GetBrushPreview _wbp_brushsetting))
  ;[1 1 1] Binding Brush Setting Widget Events and Adujusting Values of them
  (bind _result (Math|Integer|IncrementInt (Variables|Default|GetBrushTipShapeIndex))
    (:%20%20
      (if (> _result 4)
        (Variables|Default|SetBrushTipShapeIndex 0))
      (switch int (Variables|Default|GetBrushTipShapeIndex)
        (:0
          (Rendering|Material|SetTextureParameterValue _brushmaterial "BrushTipShape" "/Game/DrawingToolkit/Sources/Texture/BrushStroke/T_BasicBrush.T_BasicBrush")
          (Appearance|SetBrushfromTexture _brushpreview "/Game/DrawingToolkit/Sources/Texture/BrushStroke/T_BasicBrush_Preview.T_BasicBrush_Preview" false)
          (Rendering|Components|TextRender|SetText _brushname "Temel Firca"))
        (:1
          (Rendering|Material|SetTextureParameterValue _brushmaterial "BrushTipShape" "/Game/DrawingToolkit/Sources/Texture/BrushStroke/T_SoftBrush.T_SoftBrush")
          (Appearance|SetBrushfromTexture _brushpreview "/Game/DrawingToolkit/Sources/Texture/BrushStroke/T_SoftBrush_Preview.T_SoftBrush_Preview" false)
          (Rendering|Components|TextRender|SetText _brushname "Yumusak Firca"))
        (:2
          (Rendering|Material|SetTextureParameterValue _brushmaterial "BrushTipShape" "/Game/DrawingToolkit/Sources/Texture/BrushStroke/T_CharcoalBrush.T_CharcoalBrush")
          (Appearance|SetBrushfromTexture _brushpreview "/Game/DrawingToolkit/Sources/Texture/BrushStroke/T_CharcoalBrush_Preview.T_CharcoalBrush_Preview" false)
          (Rendering|Components|TextRender|SetText _brushname "Komur Firca"))
        (:3
          (Rendering|Material|SetTextureParameterValue _brushmaterial "BrushTipShape" "/Game/DrawingToolkit/Sources/Texture/BrushStroke/T_ChiselBrush.T_ChiselBrush")
          (Appearance|SetBrushfromTexture _brushpreview "/Game/DrawingToolkit/Sources/Texture/BrushStroke/T_ChiselBrush_Preview.T_ChiselBrush_Preview" false)
          (Rendering|Components|TextRender|SetText _brushname "Keski Firca"))
        (:4
          (Rendering|Material|SetTextureParameterValue _brushmaterial "BrushTipShape" "/Game/DrawingToolkit/Sources/Texture/BrushStroke/T_InkBrush.T_InkBrush")
          (Appearance|SetBrushfromTexture _brushpreview "/Game/DrawingToolkit/Sources/Texture/BrushStroke/T_InkBrush_Preview.T_InkBrush_Preview" false)
          (Rendering|Components|TextRender|SetText _brushname "Murekrep Firca"))))))

(event Custom|BrushTip_Left
  (bind _wbp_brushsetting (Variables|Default|GetWBP_BrushSetting))
  (bind _bp_pen (Variables|Default|GetBP%20Pen))
  (bind _brushname (Variables|/Game/DrawingToolkit/Blueprint/WidgetBP/WBP_BrushSetting.WBP_BrushSetting_C|GetBrushName _wbp_brushsetting))
  (bind _brushmaterial (Variables|/Game/DrawingToolkit/Blueprint/BP_Pen.BP_Pen_C|GetBrushMaterial _bp_pen))
  (bind _brushpreview (Variables|/Game/DrawingToolkit/Blueprint/WidgetBP/WBP_BrushSetting.WBP_BrushSetting_C|GetBrushPreview _wbp_brushsetting))
  ;[1 1 1] Binding Brush Setting Widget Events and Adujusting Values of them
  (bind _result (Math|Integer|DecrementInt (Variables|Default|GetBrushTipShapeIndex))
    (:%20%20
      (if (< _result 0)
        (Variables|Default|SetBrushTipShapeIndex 4))
      (switch int (Variables|Default|GetBrushTipShapeIndex)
        (:0
          (Rendering|Material|SetTextureParameterValue _brushmaterial "BrushTipShape" "/Game/DrawingToolkit/Sources/Texture/BrushStroke/T_BasicBrush.T_BasicBrush")
          (Appearance|SetBrushfromTexture _brushpreview "/Game/DrawingToolkit/Sources/Texture/BrushStroke/T_BasicBrush_Preview.T_BasicBrush_Preview" false)
          (Rendering|Components|TextRender|SetText _brushname "Temel Firca"))
        (:1
          (Rendering|Material|SetTextureParameterValue _brushmaterial "BrushTipShape" "/Game/DrawingToolkit/Sources/Texture/BrushStroke/T_SoftBrush.T_SoftBrush")
          (Appearance|SetBrushfromTexture _brushpreview "/Game/DrawingToolkit/Sources/Texture/BrushStroke/T_SoftBrush_Preview.T_SoftBrush_Preview" false)
          (Rendering|Components|TextRender|SetText _brushname "Yumusak Firca"))
        (:2
          (Rendering|Material|SetTextureParameterValue _brushmaterial "BrushTipShape" "/Game/DrawingToolkit/Sources/Texture/BrushStroke/T_CharcoalBrush.T_CharcoalBrush")
          (Appearance|SetBrushfromTexture _brushpreview "/Game/DrawingToolkit/Sources/Texture/BrushStroke/T_CharcoalBrush_Preview.T_CharcoalBrush_Preview" false)
          (Rendering|Components|TextRender|SetText _brushname "Komur Firca"))
        (:3
          (Rendering|Material|SetTextureParameterValue _brushmaterial "BrushTipShape" "/Game/DrawingToolkit/Sources/Texture/BrushStroke/T_ChiselBrush.T_ChiselBrush")
          (Appearance|SetBrushfromTexture _brushpreview "/Game/DrawingToolkit/Sources/Texture/BrushStroke/T_ChiselBrush_Preview.T_ChiselBrush_Preview" false)
          (Rendering|Components|TextRender|SetText _brushname "Keski Firca"))
        (:4
          (Rendering|Material|SetTextureParameterValue _brushmaterial "BrushTipShape" "/Game/DrawingToolkit/Sources/Texture/BrushStroke/T_InkBrush.T_InkBrush")
          (Appearance|SetBrushfromTexture _brushpreview "/Game/DrawingToolkit/Sources/Texture/BrushStroke/T_InkBrush_Preview.T_InkBrush_Preview" false)
          (Rendering|Components|TextRender|SetText _brushname "Murekrep Firca"))))))

(event Custom|BrushRotation
  (params (Value :type Float%20%28single-precision%29))
  (bind _returnvalue (Math|Float|MapRangeClamped Value 0.0 1.0 -1.8e+02 1.8e+02))
  ;[1 1 1] Binding Brush Setting Widget Events and Adujusting Values of them
  (Variables|/Game/DrawingToolkit/Blueprint/BP_Pen.BP_Pen_C|SetBrushRotation (Variables|Default|GetBP%20Pen) _returnvalue)
  (Class|Widget|SetRenderTransformAngle (Variables|/Game/DrawingToolkit/Blueprint/WidgetBP/WBP_BrushSetting.WBP_BrushSetting_C|GetBrushPreview (Variables|Default|GetWBP_BrushSetting)) _returnvalue))

(event Custom|Color%20Value
  (params (Value :type Float%20%28single-precision%29))
  ;[1 1 1] Binding Brush Setting Widget Events and Adujusting Values of them
  (Utilities|FlowControl|Sequence
    (:then_0
      (Variables|Default|SetColorValue Value))
    (:then_1
      ;;[1 1 1] Color Picker Event
      (bind _output_get (Variables|Default|SetX%20Aixs (stale Custom|Picker%20Color%20X X)))
      (bind _output_get_2 (Variables|Default|SetClamp%20X (Math|Float|MapRangeClamped _output_get 0.0 1.0 -1.0 1.0)))
      (Variables|Default|SetDegree (Class|KismetMathLibrary|DegAtan2 (stale _output_get_7) _output_get_2))
      (bind _output_get_3 (Variables|Default|SetCurrent%20Vector (Math|Vector2D|MakeVector2D (Variables|Default|GetClamp%20X) (Variables|Default|GetClamp%20Y))))
      (Variables|Default|SetVector%20Size (Math|Vector2D|Vector2DLength _output_get_3))
      (if (< (Variables|Default|GetDegree) 0.0)
        (bind _output_get_4 (Variables|Default|SetPicked%20Color (Class|KismetMathLibrary|HSVtoRGB (Math|Float|MapRangeClamped (Variables|Default|GetDegree) -1.8e+02 0.0 1.8e+02 3.6e+02) (Variables|Default|GetVector%20Size) (Variables|Default|GetColorValue) 1.0)))
        (Rendering|Material|SetVectorParameterValue (Variables|/Game/DrawingToolkit/Blueprint/BP_Pen.BP_Pen_C|GetBrushMaterial (Variables|Default|GetBP%20Pen)) "Brush Color" _output_get_4 :!class /Script/Engine.MaterialInstanceDynamic)
        (Class|Image|SetBrushTintColor (Variables|/Game/DrawingToolkit/Blueprint/WidgetBP/WBP_BrushSetting.WBP_BrushSetting_C|GetBrushPreview (Variables|Default|GetWBP_BrushSetting)) (Utilities|Struct|MakeSlateColor (Class|KismetMathLibrary|HSVtoRGB (Math|Float|MapRangeClamped (Variables|Default|GetDegree) -1.8e+02 0.0 1.8e+02 3.6e+02) (Variables|Default|GetVector%20Size) (Variables|Default|GetColorValue) 1.0) "UseColor_Specified"))
        (Class|Image|SetBrushTintColor (Variables|/Game/DrawingToolkit/Blueprint/WidgetBP/WBP_BrushSetting.WBP_BrushSetting_C|GetColorValueBack (Variables|Default|GetWBP_BrushSetting)) (Utilities|Struct|MakeSlateColor (Class|KismetMathLibrary|HSVtoRGB (Math|Float|MapRangeClamped (Variables|Default|GetDegree) -1.8e+02 0.0 1.8e+02 3.6e+02) (Variables|Default|GetVector%20Size) 1.0 1.0) "UseColor_Specified"))
        (else
          (bind _output_get_5 (Variables|Default|SetPicked%20Color (Class|KismetMathLibrary|HSVtoRGB (Variables|Default|GetDegree) (Variables|Default|GetVector%20Size) (Variables|Default|GetColorValue) 1.0)))
          (Rendering|Material|SetVectorParameterValue (Variables|/Game/DrawingToolkit/Blueprint/BP_Pen.BP_Pen_C|GetBrushMaterial (Variables|Default|GetBP%20Pen)) "Brush Color" _output_get_5 :!class /Script/Engine.MaterialInstanceDynamic)
          (Class|Image|SetBrushTintColor (Variables|/Game/DrawingToolkit/Blueprint/WidgetBP/WBP_BrushSetting.WBP_BrushSetting_C|GetBrushPreview (Variables|Default|GetWBP_BrushSetting)) (Utilities|Struct|MakeSlateColor (Class|KismetMathLibrary|HSVtoRGB (Variables|Default|GetDegree) (Variables|Default|GetVector%20Size) (Variables|Default|GetColorValue) 1.0) "UseColor_Specified"))
          (Class|Image|SetBrushTintColor (Variables|/Game/DrawingToolkit/Blueprint/WidgetBP/WBP_BrushSetting.WBP_BrushSetting_C|GetColorValueBack (Variables|Default|GetWBP_BrushSetting)) (Utilities|Struct|MakeSlateColor (Class|KismetMathLibrary|HSVtoRGB (Variables|Default|GetDegree) (Variables|Default|GetVector%20Size) 1.0 1.0) "UseColor_Specified")))))
    (:then_2
      (bind _output_get_6 (Variables|Default|SetY%20Aixs (* (stale Custom|Picker%20Color%20Y Y) -1.0)))
      (bind _output_get_7 (Variables|Default|SetClamp%20Y (Math|Float|MapRangeClamped _output_get_6 0.0 -1.0 -1.0 1.0))))))

(event EventBeginPlay
  ;[1 1 1] Begin Play
  (Utilities|FlowControl|Sequence
    (:then_0
      (Transformation|SetRelativeRotation (Variables|Default|GetDotPoint) (Math|Rotator|MakeRotator 0.0 0.0 3.0) false false))
    (:then_1
      (bind _outactors (Actor|GetAllActorsOfClass "/Game/DrawingToolkit/Blueprint/BP_Pen.BP_Pen_C"))
      (Variables|Default|SetBP%20Pen (Utilities|Array|Get(acopy) _outactors)))
    (:then_2
      (bind _returnvalue (UserInterface|CreateWidget "/Game/DrawingToolkit/Blueprint/WidgetBP/WBP_BrushSetting.WBP_BrushSetting_C"))
      (bind _output_get (Variables|Default|SetWBP_BrushSetting _returnvalue))
      (UserInterface|SetWidget (Variables|Default|GetWidget) _output_get)
      ;[1 1 1] Binding Brush Setting Widget Events and Adujusting Values of them
      (EventDispatchers|BindEventtoOnValueChanged (Variables|/Game/DrawingToolkit/Blueprint/WidgetBP/WBP_BrushSetting.WBP_BrushSetting_C|GetSliderBar_Size (Variables|Default|GetWBP_BrushSetting)) (delegate Custom|BrushSize))
      (EventDispatchers|BindEventtoOnValueChanged (Variables|/Game/DrawingToolkit/Blueprint/WidgetBP/WBP_BrushSetting.WBP_BrushSetting_C|GetSliderBar_Opacity (Variables|Default|GetWBP_BrushSetting)) (delegate Custom|BrushOpacity))
      (EventDispatchers|BindEventtoOnClicked (Variables|/Game/DrawingToolkit/Blueprint/WidgetBP/WBP_BrushSetting.WBP_BrushSetting_C|GetBrushTip_RightButton (Variables|Default|GetWBP_BrushSetting)) (delegate Custom|BrushTip_Right))
      (EventDispatchers|BindEventtoOnClicked (Variables|/Game/DrawingToolkit/Blueprint/WidgetBP/WBP_BrushSetting.WBP_BrushSetting_C|GetBrushTip_LeftButton (Variables|Default|GetWBP_BrushSetting)) (delegate Custom|BrushTip_Left))
      (EventDispatchers|BindEventtoOnValueChanged (Variables|/Game/DrawingToolkit/Blueprint/WidgetBP/WBP_BrushSetting.WBP_BrushSetting_C|GetSliderBar_Rotation (Variables|Default|GetWBP_BrushSetting)) (delegate Custom|BrushRotation))
      (EventDispatchers|BindEventtoOnValueChanged (Variables|/Game/DrawingToolkit/Blueprint/WidgetBP/WBP_BrushSetting.WBP_BrushSetting_C|GetSliderBar_ColorValue (Variables|Default|GetWBP_BrushSetting)) (delegate Custom|Color%20Value)))))

(event EventTick
  (params (DeltaSeconds :type Float%20%28single-precision%29))
  (bind _bp_pen (Variables|Default|GetBP%20Pen))
  ;[1 1 1] VR Version
  (if (Variables|/Game/DrawingToolkit/Blueprint/BP_Pen.BP_Pen_C|GetColor%20Picked _bp_pen)
    (Transformation|SetRelativeLocation (Variables|Default|GetDotPoint) (Math|Vector|MakeVector (Math|Float|MapRangeClamped (Variables|/Game/DrawingToolkit/Blueprint/BP_Pen.BP_Pen_C|GetPicked%20Color%20X _bp_pen) 0.0 1.0 -5e+01 5e+01) (Math|Float|MapRangeClamped (Variables|/Game/DrawingToolkit/Blueprint/BP_Pen.BP_Pen_C|GetPicked%20Color%20Y _bp_pen) 0.0 1.0 -5e+01 5e+01) 4.0) false false)))

(fn ConstructionScript)