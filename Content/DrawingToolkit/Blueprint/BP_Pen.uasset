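; BP_Pen is a tracked pen that paints and erases on drawing panels.
; Each Tick remaps the LiveLinkVive actor's X and Z into pen position on a fixed Y plane.
; While the first-person character's Click is set, a -Y trace draws brush materials into panel render targets at the hit UV, using a second material for EraseMode.
; The trace also feeds color picks to BP_BrushSetting and, outside erase mode, drags BP_Horn.
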(event EventBeginPlay
  ;[1 1 1] Pen BeginPlay
  (Utilities|FlowControl|Sequence
    (:then_0
      (Input|EnableInput (Game|GetPlayerController 0)))
    (:then_1
      (bind _outactors (Actor|GetAllActorsOfClass "/Game/DrawingToolkit/Blueprint/VirtualRealityBP/BP_MotionControllerPawnVR.BP_MotionControllerPawnVR_C"))
      (Variables|Default|SetMotionController (Utilities|Array|Get(acopy) _outactors)))
    (:then_2
      (bind _returnvalue (Rendering|Material|CreateDynamicMaterialInstance "/Game/DrawingToolkit/Sources/Material/M_Brush.M_Brush" "None" "None" :!class /Script/Engine.KismetMaterialLibrary))
      (Variables|Default|SetBrushMaterial _returnvalue))
    (:then_3
      (bind _outactors_2 (Actor|GetAllActorsOfClass "/Game/DrawingToolkit/Blueprint/BP_DrawingPanel.BP_DrawingPanel_C"))
      (Variables|Default|SetDrawingArea _outactors_2))
    (:then_4
      (bind _returnvalue_2 (Rendering|Material|CreateDynamicMaterialInstance "/Game/DrawingToolkit/Sources/Material/M_Brush2.M_Brush2" "None" "None" :!class /Script/Engine.KismetMaterialLibrary))
      (Variables|Default|SetBrushMaterial2 _returnvalue_2))))

(event EventTick
  (params (DeltaSeconds :type Float%20%28single-precision%29))
  (bind _cylinder (Variables|Default|GetCylinder))
  (bind _staticmesh (Variables|Default|GetStaticMesh))
  (bind _returnvalue (Transformation|GetWorldLocation _cylinder))
  (bind _returnvalue_2 (Transformation|GetWorldLocation _staticmesh))
  (bind _returnvalue_3 (+ _returnvalue_2 "0.000000,-1000.000000,0.000000"))
  (Utilities|FlowControl|Sequence
    (:then_0
      ;[1 1 1] Start Drawing on Drawing Area
      (if (Variables|/Game/DrawingToolkit/Blueprint/BP_FirstPersonCharacter.BP_FirstPersonCharacter_C|GetClick (.AsBP%20First%20Person%20Character (Utilities|Casting|CastToBP_FirstPersonCharacter (Game|GetPlayerCharacter 0))))
        (if (Variables|Default|GetEraseMode)
          ;[1 1 1] Erase
          (bind (_outhit _returnvalue_4) (Collision|LineTraceByChannel _returnvalue_2 _returnvalue_3 "TraceTypeQuery1" true 0 "None" true "(R=0.845486,G=0.000000,B=0.022773,A=1.000000)"))
          (Utilities|FlowControl|Sequence
            (:then_0
              (if _returnvalue_4
                (for _array_element (Variables|Default|GetDrawingArea)
                  (if (== (.HitActor (Collision|BreakHitResult _outhit)) _array_element)
                    (bind (_canvas _size _context) (Rendering|BeginDrawCanvastoRenderTarget (Variables|/Game/DrawingToolkit/Blueprint/BP_DrawingPanel.BP_DrawingPanel_C|GetRenderTarget _array_element)))
                    (Canvas|DrawMaterial _canvas (Variables|Default|GetBrushMaterial2) (.Screen%20Position (CallFunction|SetCanvasMaterialScaleandPosition _size (Math|Vector2D|MakeVector2D (.X (Math|Vector2D|BreakVector2D (.UV (Class|GameplayStatics|FindCollisionUV _outhit)))) (.Y (Math|Vector2D|BreakVector2D (.UV (Class|GameplayStatics|FindCollisionUV _outhit))))) (/ (/ (Variables|Default|GetBrushSize) 2.0) (.x (Transformation|GetWorldScale (Variables|/Game/DrawingToolkit/Blueprint/BP_DrawingPanel.BP_DrawingPanel_C|GetDrawingArea _array_element)))))) (Math|Vector2D|MakeVector2D (/ (.X (Math|Vector2D|BreakVector2D (.Screen%20Size (CallFunction|SetCanvasMaterialScaleandPosition _size (Math|Vector2D|MakeVector2D (.X (Math|Vector2D|BreakVector2D (.UV (Class|GameplayStatics|FindCollisionUV _outhit)))) (.Y (Math|Vector2D|BreakVector2D (.UV (Class|GameplayStatics|FindCollisionUV _outhit))))) (/ (/ (Variables|Default|GetBrushSize) 2.0) (.x (Transformation|GetWorldScale (Variables|/Game/DrawingToolkit/Blueprint/BP_DrawingPanel.BP_DrawingPanel_C|GetDrawingArea _array_element)))))))) 1.5) (.Y (Math|Vector2D|BreakVector2D (.Screen%20Size (CallFunction|SetCanvasMaterialScaleandPosition _size (Math|Vector2D|MakeVector2D (.X (Math|Vector2D|BreakVector2D (.UV (Class|GameplayStatics|FindCollisionUV _outhit)))) (.Y (Math|Vector2D|BreakVector2D (.UV (Class|GameplayStatics|FindCollisionUV _outhit))))) (/ (/ (Variables|Default|GetBrushSize) 2.0) (.x (Transformation|GetWorldScale (Variables|/Game/DrawingToolkit/Blueprint/BP_DrawingPanel.BP_DrawingPanel_C|GetDrawingArea _array_element))))))))) "(X=0.000000,Y=0.000000)" "(X=1.000000,Y=1.000000)" (Variables|Default|GetBrushRotation) "(X=0.500000,Y=0.500000)")
                    (Rendering|EndDrawCanvastoRenderTarget _context)))))
            (:then_1
              (if _returnvalue_4
                (bind _asbp_brush_setting (Utilities|Casting|CastToBP_BrushSetting (.HitActor (Collision|BreakHitResult _outhit))))
                (if (!= (Variables|/Game/DrawingToolkit/Blueprint/BP_BrushSetting.BP_BrushSetting_C|GetWidget _asbp_brush_setting) (.HitComponent (Collision|BreakHitResult _outhit)))
                  (Utilities|FlowControl|Sequence
                    (:then_0
                      (bind _output_get (Variables|Default|SetPicked%20Color%20X (.X (Math|Vector2D|BreakVector2D (.UV (Class|GameplayStatics|FindCollisionUV _outhit))))))
                      (Default|PickerColorX _asbp_brush_setting _output_get))
                    (:then_1
                      (bind _output_get_2 (Variables|Default|SetPicked%20Color%20Y (.Y (Math|Vector2D|BreakVector2D (.UV (Class|GameplayStatics|FindCollisionUV _outhit))))))
                      (Default|PickerColorY _asbp_brush_setting _output_get_2)))))))
          (else
            (Variables|Default|SetColor%20Picked true)
            (bind (_outhit_2 _returnvalue_5) (Collision|LineTraceByChannel _returnvalue_2 _returnvalue_3 "TraceTypeQuery1" true 0 "None" true "(R=0.845486,G=0.000000,B=0.022773,A=1.000000)"))
            (Utilities|FlowControl|Sequence
              (:then_0
                (if _returnvalue_5
                  (if (not (Variables|Default|GetIsMovingAnything))
                    (for _array_element_2 (Variables|Default|GetDrawingArea)
                      (if (== (.HitActor (Collision|BreakHitResult _outhit_2)) _array_element_2)
                        (bind (_canvas_2 _size_2 _context_2) (Rendering|BeginDrawCanvastoRenderTarget (Variables|/Game/DrawingToolkit/Blueprint/BP_DrawingPanel.BP_DrawingPanel_C|GetRenderTarget _array_element_2)))
                        (Canvas|DrawMaterial _canvas_2 (Variables|Default|GetBrushMaterial) (.Screen%20Position (CallFunction|SetCanvasMaterialScaleandPosition _size_2 (Math|Vector2D|MakeVector2D (.X (Math|Vector2D|BreakVector2D (.UV (Class|GameplayStatics|FindCollisionUV _outhit_2)))) (.Y (Math|Vector2D|BreakVector2D (.UV (Class|GameplayStatics|FindCollisionUV _outhit_2))))) (/ (Variables|Default|GetBrushSize) (.x (Transformation|GetWorldScale (Variables|/Game/DrawingToolkit/Blueprint/BP_DrawingPanel.BP_DrawingPanel_C|GetDrawingArea _array_element_2)))))) (.Screen%20Size (CallFunction|SetCanvasMaterialScaleandPosition _size_2 (Math|Vector2D|MakeVector2D (.X (Math|Vector2D|BreakVector2D (.UV (Class|GameplayStatics|FindCollisionUV _outhit_2)))) (.Y (Math|Vector2D|BreakVector2D (.UV (Class|GameplayStatics|FindCollisionUV _outhit_2))))) (/ (Variables|Default|GetBrushSize) (.x (Transformation|GetWorldScale (Variables|/Game/DrawingToolkit/Blueprint/BP_DrawingPanel.BP_DrawingPanel_C|GetDrawingArea _array_element_2)))))) "(X=0.000000,Y=0.000000)" "(X=1.000000,Y=1.000000)" (- (Variables|Default|GetBrushRotation) -9e+01) "(X=0.500000,Y=0.500000)")
                        (Rendering|EndDrawCanvastoRenderTarget _context_2))))))
              (:then_1
                (if _returnvalue_5
                  (if (not (Variables|Default|GetIsMovingAnything))
                    (bind _asbp_brush_setting_2 (Utilities|Casting|CastToBP_BrushSetting (.HitActor (Collision|BreakHitResult _outhit_2))))
                    (if (!= (Variables|/Game/DrawingToolkit/Blueprint/BP_BrushSetting.BP_BrushSetting_C|GetWidget _asbp_brush_setting_2) (.HitComponent (Collision|BreakHitResult _outhit_2)))
                      (Utilities|FlowControl|Sequence
                        (:then_0
                          (bind _output_get_3 (Variables|Default|SetPicked%20Color%20X (.X (Math|Vector2D|BreakVector2D (.UV (Class|GameplayStatics|FindCollisionUV _outhit_2))))))
                          (Default|PickerColorX _asbp_brush_setting_2 _output_get_3))
                        (:then_1
                          (bind _output_get_4 (Variables|Default|SetPicked%20Color%20Y (.Y (Math|Vector2D|BreakVector2D (.UV (Class|GameplayStatics|FindCollisionUV _outhit_2))))))
                          (Default|PickerColorY _asbp_brush_setting_2 _output_get_4)))))))
              (:then_2
                (if _returnvalue_5
                  (bind _asbp_horn (Utilities|Casting|CastToBP_Horn (.HitActor (Collision|BreakHitResult _outhit_2))))
                  (if (== (Variables|/Game/MyStuff/Drawable/BP_Horn.BP_Horn_C|GetPlane _asbp_horn) (.HitComponent (Collision|BreakHitResult _outhit_2)))
                    (Variables|Default|SetIsMovingAnything true)
                    (Transformation|SetActorLocation _asbp_horn (Math|Vector|MakeVector (.x _returnvalue) 92.0 (+ (.z _returnvalue) -1.1e+02)) false false)))))))
        (else
          (Variables|Default|SetIsMovingAnything false))))
    (:then_1
      (bind _returnvalue_6 (Actor|GetActorOfClass "/Game/LiveLinkVive.LiveLinkVive_C"))
      (bind _new_value (CallFunction|Optimizer (.x (Transformation|GetWorldLocation (Variables|/Game/LiveLinkVive.LiveLinkVive_C|GetDefaultSceneRoot _returnvalue_6))) 3e+02 137.0 -1167.0 -2076.0))
      (bind _new_value_2 (CallFunction|Optimizer (.z (Transformation|GetWorldLocation (Variables|/Game/LiveLinkVive.LiveLinkVive_C|GetDefaultSceneRoot _returnvalue_6))) 4e+01 1.2e+02 827.0 317.0))
      (Transformation|SetActorLocation (Math|Vector|MakeVector _new_value 4e+02 _new_value_2) false false))))

(event Input|ActionEvents|InputActionTrackingAction
  (params (Key :type Key%20Structure :default "None"))
  (:Pressed
    (Development|PrintString "yesss"))
  (:Released
    (Development|PrintString "Hello")))

(fn ConstructionScript)

(fn ReleaseParticle)

(fn Optimizer
  (params (Current%20Value :type Float%20%28double-precision%29) (Min%20value :type Float%20%28double-precision%29) (Max%20value :type Float%20%28double-precision%29) (Max%20range%20%20 :type Float%20%28double-precision%29) (min%20range :type Float%20%28double-precision%29))
  (return (+ (* (/ (- Current%20Value Min%20value) (- Max%20value Min%20value)) (- Max%20range%20%20 min%20range)) min%20range)))